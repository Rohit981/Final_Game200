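; Paper2D player character that walks on world axes, swaps idle and walk flipbooks by facing, and interacts with objects in front of it.
; Each tick it derives a four-way direction from input, snaps control rotation to match, and sphere-traces ahead from the capsule's forward vector.
; Hits on InteractableObjects set a visibility flag and pass the object's interface name to a HUD widget.
; While that flag is set, Interact shows the HUD and mouse cursor.
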(event EventBeginPlay
  ;[1 1 1] Initialize the interaction HUD
  (bind _returnvalue (UserInterface|CreateWidget "/Game/UI/Interaction_HUD.Interaction_HUD_C"))
  (Variables|Default|SetInteraction_HUD_Ref _returnvalue))

(event EventTick
  (params (DeltaSeconds :type Float%20%28single-precision%29))
  ;[1 1 1] Draw Ray & Set Player Rotation
  (CallFunction|SetAnimations)
  (CallFunction|InteractionCheck)
  (CallFunction|SetSpriteRotationForward)
  (CallFunction|SetSpriteRotationLeft))

(event Input|ActionEvents|InputActionInteract
  (params (Key :type Key%20Structure :default "None"))
  ;[1 1 1] Interaction
  (:Pressed
    (CallFunction|Interaction)))

(event Input|AxisEvents|InputAxisMoveRight
  (params (AxisValue :type Float%20%28single-precision%29))
  ;[1 1 1] Back&Forward Movement
  (Pawn|Input|AddMovementInput "1.000000, 0,0.000000" AxisValue false))

(event Input|AxisEvents|InputAxisMoveUp
  (params (AxisValue :type Float%20%28single-precision%29))
  ;[1 1 1] Left&RightMovement
  (Pawn|Input|AddMovementInput "0,-1.000000,0.000000" AxisValue false))

(fn ConstructionScript)

(fn SetAnimations
  (if (or (!= (Input|AxisValues|GetMoveRight) 0.0) (!= (Input|AxisValues|GetMoveUp) 0.0))
    (bind _output_get (Variables|Default|SetPlayerDirections (select (> (Input|AxisValues|GetMoveRight) 0.0) "NewEnumerator0" (select (< (Input|AxisValues|GetMoveRight) 0.0) "NewEnumerator1" (select (> (Input|AxisValues|GetMoveUp) 0.0) "NewEnumerator2" "NewEnumerator3"))))))
  (Sprite|SetFlipbook (Variables|Default|GetSprite) (select (> (Math|Vector|VectorLength (Transformation|GetVelocity)) 0.0) (Utilities|Select :Index _output_get :NewEnumerator0 "/Game/2DAssets/Animations/Character/Move_Forward.Move_Forward" :NewEnumerator1 "/Game/2DAssets/Animations/Character/Move_Backward.Move_Backward" :NewEnumerator2 "/Game/2DAssets/Animations/Character/Move_Left.Move_Left" :NewEnumerator3 "/Game/2DAssets/Animations/Character/Move_Right.Move_Right") (Utilities|Select :Index _output_get :NewEnumerator0 "/Game/2DAssets/Animations/Character/Character_Idle_Forward.Character_Idle_Forward" :NewEnumerator1 "/Game/2DAssets/Animations/Character/Character_Backward_Idle.Character_Backward_Idle" :NewEnumerator2 "/Game/2DAssets/Animations/Character/Character_Left_Idle.Character_Left_Idle" :NewEnumerator3 "/Game/2DAssets/Animations/Character/Character_Right_Idle.Character_Right_Idle"))))

(fn InteractionCheck
  (bind _returnvalue (Transformation|GetActorLocation))
  (bind (_outhit _returnvalue_2) (Collision|SphereTraceByChannel _returnvalue (+ _returnvalue (* (Math|Vector|GetForwardVector (Transformation|GetWorldRotation (Variables|Collision|GetCapsuleComponent))) 5e+01)) 1e+01 "TraceTypeQuery3" false 0 "None"))
  (if _returnvalue_2
    (bind _asinteractable_objects (Utilities|Casting|CastToInteractableObjects (.hitactor _outhit)))
    (bind _output_get (Variables|/Game/Blueprints/InteractableObjects.InteractableObjects_C|SetCheckVisibilty _asinteractable_objects true))
    (Variables|Default|SetUI_Visible? _output_get)
    (if (Utilities|DoesObjectImplementInterface (.hitactor _outhit) "/Game/Blueprints/GetObjectName_Interface.GetObjectName_Interface_C")
      (bind _name (Class|GetObjectNameInterface|GetName(Message) (.hitactor _outhit)))
      (Variables|/Game/UI/Interaction_HUD.Interaction_HUD_C|SetObjectName (Variables|Default|GetInteraction_HUD_Ref) _name))
    (else
      (Variables|Default|SetUI_Visible? false))))

(fn SetSpriteRotationForward
  (if (Utilities|Select :Index (Variables|Default|GetPlayerDirections) :NewEnumerator0 true :NewEnumerator1 false :NewEnumerator2 false :NewEnumerator3 false)
    (Pawn|SetControlRotation (Pawn|GetController) (Math|Rotator|MakeRotator 0.0 0.0 0.0))
    (elif (Utilities|Select :Index (Variables|Default|GetPlayerDirections) :NewEnumerator0 false :NewEnumerator1 true :NewEnumerator2 false :NewEnumerator3 false)
      (Pawn|SetControlRotation (Pawn|GetController) (Math|Rotator|MakeRotator 0.0 0.0 1.8e+02)))))

(fn SetSpriteRotationLeft
  (if (Utilities|Select :Index (Variables|Default|GetPlayerDirections) :NewEnumerator0 false :NewEnumerator1 false :NewEnumerator2 false :NewEnumerator3 true)
    (Pawn|SetControlRotation (Pawn|GetController) (Math|Rotator|MakeRotator 0.0 0.0 9e+01))
    (elif (Utilities|Select :Index (Variables|Default|GetPlayerDirections) :NewEnumerator0 false :NewEnumerator1 false :NewEnumerator2 true :NewEnumerator3 false)
      (Pawn|SetControlRotation (Pawn|GetController) (Math|Rotator|MakeRotator 0.0 0.0 -9e+01)))))

(fn Interaction
  (bind _returnvalue (Game|GetPlayerController 0))
  (if (Variables|Default|GetUI_Visible?)
    (UserInterface|Viewport|AddtoViewport (Variables|Default|GetInteraction_HUD_Ref) 0)
    (Input|SetInputModeGameandUI _returnvalue 0 "DoNotLock" true)
    (Variables|/Script/Engine.PlayerController|SetbShowMouseCursor _returnvalue true)))