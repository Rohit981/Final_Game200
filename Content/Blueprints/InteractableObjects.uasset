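; Interactable sprite object that shows an interaction UI and changes its sprite when the player interacts with it.
; Each tick it reads the player pawn's UIVisible flag, showing the UI only while its own CheckVisibilty flag is also set, and hiding it and clearing that flag otherwise.
; On IsInteracted, a visible object swaps to InteractableSprite and hides the UI.
; GetName exposes the object's Name.
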(event EventTick
  (params (DeltaSeconds :type Float%20%28single-precision%29))
  (bind _interactionui (Variables|Default|GetInteractionUI))
  ;[1 1 1] Setting the Interaction UI visibilty based on the Raycast hit check
  (bind _asplayer_bp (Utilities|Casting|CastToPlayer_BP (Game|Player|GetPlayerPawn 0)))
  (if (Variables|/Game/Blueprints/Player_BP.Player_BP_C|GetUI_Visible? _asplayer_bp)
    (if (Variables|Default|GetCheckVisibilty)
      (Development|SetHiddeninGame _interactionui false false)
      (if (Variables|/Game/Blueprints/Player_BP.Player_BP_C|GetIsInteracted? _asplayer_bp)
        (Rendering|Components|Sprite|SetSprite (Variables|Default|GetRenderComponent) (Variables|Default|GetInteractableSprite))
        (Development|SetHiddeninGame _interactionui true false)))
    (else
      (Variables|Default|SetCheckVisibilty false)
      (Development|SetHiddeninGame _interactionui true false))))

(fn ConstructionScript)

(fn GetName
  (return (Variables|Default|GetName)))